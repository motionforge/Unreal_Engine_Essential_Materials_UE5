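; Cube box-mask actor that publishes its static mesh's world transform to the MPC_Masking_Area material parameter collection.
; It writes world location and scale to the collection's Location and Scale vector parameters; rotation is not passed.
; The construction script does this when the actor is constructed, and Tick repeats it every frame so the parameters follow the moving or scaled mesh.
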(event EventBeginPlay)

(event Collision|EventActorBeginOverlap
  (params (OtherActor :type Actor%20Object%20Reference)))

(event EventTick
  (params (DeltaSeconds :type Float%20%28single-precision%29))
  (bind _staticmeshcomponent (Variables|Debug|GetStaticMeshComponent))
  (Rendering|Material|SetVectorParameterValue "/Game/Material/Masking_Materials/MPC_Masking_Area.MPC_Masking_Area" "Location" (Math|Conversions|ToLinearColor(Vector) (Transformation|GetWorldLocation _staticmeshcomponent)) :!class /Script/Engine.KismetMaterialLibrary)
  (Rendering|Material|SetVectorParameterValue "/Game/Material/Masking_Materials/MPC_Masking_Area.MPC_Masking_Area" "Scale" (Math|Conversions|ToLinearColor(Vector) (Transformation|GetWorldScale _staticmeshcomponent)) :!class /Script/Engine.KismetMaterialLibrary))

(fn ConstructionScript
  (bind _staticmeshcomponent (Variables|Debug|GetStaticMeshComponent))
  (Rendering|Material|SetVectorParameterValue "/Game/Material/Masking_Materials/MPC_Masking_Area.MPC_Masking_Area" "Location" (Math|Conversions|ToLinearColor(Vector) (Transformation|GetWorldLocation _staticmeshcomponent)) :!class /Script/Engine.KismetMaterialLibrary)
  (Rendering|Material|SetVectorParameterValue "/Game/Material/Masking_Materials/MPC_Masking_Area.MPC_Masking_Area" "Scale" (Math|Conversions|ToLinearColor(Vector) (Transformation|GetWorldScale _staticmeshcomponent)) :!class /Script/Engine.KismetMaterialLibrary))